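; Triangle switch tile that opens a path when the player character (PC_BP) overlaps it.
; On overlap it runs the parent's overlap logic, then destroys the first Tile_Gate_Triangle found in the level.
; It then spawns a Tile00_Bridge at a hardcoded transform, so the result is tied to one specific level layout.
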(event `self.ReceiveActorBeginOverlap`
  (params (OtherActor :type "Actor Object Reference"))
  (bind _aspc_bp (cast `/Game/PuzzleBP/Blueprints/PC_BP` OtherActor))
  (`parent.ReceiveActorBeginOverlap` _aspc_bp)
  (bind _outactors (`GameplayStatics.GetAllActorsOfClass` "/Game/Blueprints/Tile_Gate_Triangle.Tile_Gate_Triangle_C"))
  (`self.K2_DestroyActor` (`|GetArrayItem` _outactors))
  (`|SpawnActorFromClass` "/Game/Blueprints/Tile00_Bridge.Tile00_Bridge_C" (`KismetMathLibrary.MakeTransform` (-550.0 350.0 40.0)) "Undefined" "OverrideRootScale" null null))

(fn `UserConstructionScript`
  (`parent.UserConstructionScript`))