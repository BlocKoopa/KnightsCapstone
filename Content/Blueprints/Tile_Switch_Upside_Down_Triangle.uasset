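; Switch tile that opens the upside-down triangle torii gate when the player's chess piece (PC_BP_Chess) overlaps it.
; On overlap it runs the parent tile's overlap logic, then destroys the first Tile_Torii_Upside_Down_Triangle found in the level.
; It spawns a Tile_Torii_Open at a hard-coded transform, with no check that a closed gate still exists.
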(event `self.ReceiveActorBeginOverlap`
  (params (OtherActor :type "Actor Object Reference"))
  (bind _aspc_bp_chess (cast `/Game/PuzzleBP/Blueprints/PC_BP_Chess` OtherActor))
  (`parent.ReceiveActorBeginOverlap` _aspc_bp_chess)
  (bind _outactors (`GameplayStatics.GetAllActorsOfClass` "/Game/Blueprints/Tile_Torii_Upside_Down_Triangle.Tile_Torii_Upside_Down_Triangle_C"))
  (`self.K2_DestroyActor` (`|GetArrayItem` _outactors))
  (`|SpawnActorFromClass` "/Game/Blueprints/Tile_Torii_Open.Tile_Torii_Open_C" (`KismetMathLibrary.MakeTransform` (-3950.0 5750.0 50.0) (struct :`Yaw` 90.0)) "Undefined" "OverrideRootScale" null null))

(fn `UserConstructionScript`
  (`parent.UserConstructionScript`))