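; Switch tile actor that opens a gate when the player pawn (PC_BP) steps onto it.
; On overlap it destroys the first Tile_Gate_Square found in the level and spawns a Tile00 at a hard-coded world position, presumably filling the gap.
; The parent overlap logic runs first, and nothing prevents the switch from firing again on later overlaps.
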(event `self.ReceiveActorBeginOverlap`
  (params (OtherActor :type "Actor Object Reference"))
  (bind _aspc_bp (cast `/Game/PuzzleBP/Blueprints/PC_BP` OtherActor))
  (`parent.ReceiveActorBeginOverlap` _aspc_bp)
  (bind _outactors (`GameplayStatics.GetAllActorsOfClass` "/Game/Blueprints/Tile_Gate_Square.Tile_Gate_Square_C"))
  (`self.K2_DestroyActor` (`|GetArrayItem` _outactors))
  (`|SpawnActorFromClass` "/Game/Blueprints/Tile00.Tile00_C" (`KismetMathLibrary.MakeTransform` (50.0 -1450.0 40.0) (struct)) "Undefined" "OverrideRootScale" null null))

(fn `UserConstructionScript`
  (`parent.UserConstructionScript`))