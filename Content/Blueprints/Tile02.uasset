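; Puzzle board tile that turns blue and clickable when the PC_BP piece is an L-shaped move away, two steps in X and one in Y.
; A movable Checker component probes four such paths with delays, requiring tagged tiles along each before testing for the piece.
; Clicking or touching a clickable tile increments player score, moves the piece above it and makes every Tile02 rerun the probe.
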(event `self.StaticMesh.OnClicked`
  (params (TouchedComponent :type "PrimitiveComponent Object Reference") (ButtonPressed :type "Key Structure"))
  (if (`self.Clickable`) :!label _label
    (`/Engine/EditorBlueprintResources/StandardMacros.IncrementInt` (`/Game/PuzzleBP/Blueprints/PuzzlePlayerCharacter.Score` (`self.MuhCharacdor`))
      (:`  `
        (bind _outactors (`GameplayStatics.GetAllActorsOfClass` "/Game/PuzzleBP/Blueprints/PC_BP.PC_BP_C"))
        (`self.K2_SetActorRelativeLocation` (`|GetArrayItem` _outactors) (`KismetMathLibrary.MakeVector` (.x (`SceneComponent.K2_GetComponentLocation` (`self.DefaultSceneRoot`))) (.y (`SceneComponent.K2_GetComponentLocation` (`self.DefaultSceneRoot`))) (+ (.z (`SceneComponent.K2_GetComponentLocation` (`self.DefaultSceneRoot`))) 40.0)) false false)
        (bind _outactors_2 (`GameplayStatics.GetAllActorsOfClass` "Tile02_C"))
        (for _array_element _outactors_2
          (`self.ResetTile02` _array_element))))))

(event `self.StaticMesh.OnInputTouchBegin`
  (params (FingerIndex :type "ETouchIndex Enum" :default "Touch1") (TouchedComponent :type "PrimitiveComponent Object Reference"))
  (goto _label))

(event `ResetTile02`
  (bind _checker (`self.Checker`))
  (bind _checker_2 (`self.Checker`))
  (bind _checker_3 (`self.Checker`))
  (bind _checker_4 (`self.Checker`))
  (set `self.Clickable` false)
  ;[1 1 1] Y RIGHT 300
  (`SceneComponent.K2_SetWorldLocation` (`self.Checker`) (`KismetMathLibrary.MakeVector` (.x (`SceneComponent.K2_GetComponentLocation` (`self.DefaultSceneRoot`))) (+ (.y (`SceneComponent.K2_GetComponentLocation` (`self.DefaultSceneRoot`))) 300.0) (.z (`SceneComponent.K2_GetComponentLocation` (`self.DefaultSceneRoot`)))) false false :!label _label_2)
  (`KismetSystemLibrary.Delay` (`self.Delay`))
  ;[1 1 1] TILE????
  (if (`KismetStringLibrary.Contains` (`KismetSystemLibrary.GetDisplayName` (`|GetArrayItem` (`self.GetComponentsByTag` (`|GetArrayItem` (`PrimitiveComponent.GetOverlappingActors` (`self.Checker`) "Tile02_C")) "/Script/Engine.StaticMeshComponent" "Tile"))) "Static")
    ;[1 1 1] X DOWN 300
    (`SceneComponent.K2_SetWorldLocation` (`self.Checker`) (`KismetMathLibrary.MakeVector` (+ (.x (`SceneComponent.K2_GetComponentLocation` (`self.Checker`))) -300.0) (.y (`SceneComponent.K2_GetComponentLocation` (`self.Checker`))) (.z (`SceneComponent.K2_GetComponentLocation` (`self.Checker`)))) false false)
    ;[1 1 1] TILE????
    (if (`KismetStringLibrary.Contains` (`KismetSystemLibrary.GetDisplayName` (`|GetArrayItem` (`self.GetComponentsByTag` (`|GetArrayItem` (`PrimitiveComponent.GetOverlappingActors` (`self.Checker`) "Tile02_C")) "/Script/Engine.StaticMeshComponent" "Tile"))) "Static")
      ;[1 1 1] X DOWN 600
      (`SceneComponent.K2_SetWorldLocation` (`self.Checker`) (`KismetMathLibrary.MakeVector` (+ (.x (`SceneComponent.K2_GetComponentLocation` (`self.Checker`))) -300.0) (.y (`SceneComponent.K2_GetComponentLocation` (`self.Checker`))) (.z (`SceneComponent.K2_GetComponentLocation` (`self.Checker`)))) false false)
      (bind (_outactors _returnvalue) (`KismetSystemLibrary.ComponentOverlapActors` _checker (`SceneComponent.K2_GetComponentToWorld` _checker) (`self.TypeSelected`) "/Game/PuzzleBP/Blueprints/PC_BP.PC_BP_C"))
      ;[1 1 1] PLAYER???
      (if _returnvalue
        (set `self.Clickable` true)
        ;[1 1 1] SET MAT T/F
        (`PrimitiveComponent.SetMaterial` (`self.StaticMesh`) 0 "/Game/Puzzle/Meshes/BlueMaterial.BlueMaterial")
        (else
          (`PrimitiveComponent.SetMaterial` (`self.StaticMesh`) 0 "/Game/Materials/M_Main_I_Tan.M_Main_I_Tan")
          (`KismetSystemLibrary.PrintString` "" :!label _label_3)
          ;[1 1 1] Y RIGHT 300
          (`SceneComponent.K2_SetWorldLocation` (`self.Checker`) (`KismetMathLibrary.MakeVector` (.x (`SceneComponent.K2_GetComponentLocation` (`self.DefaultSceneRoot`))) (+ (.y (`SceneComponent.K2_GetComponentLocation` (`self.DefaultSceneRoot`))) 300.0) (.z (`SceneComponent.K2_GetComponentLocation` (`self.DefaultSceneRoot`)))) false false)
          (`KismetSystemLibrary.Delay` (`self.Delay`))
          ;[1 1 1] TILE????
          (if (`KismetStringLibrary.Contains` (`KismetSystemLibrary.GetDisplayName` (`|GetArrayItem` (`self.GetComponentsByTag` (`|GetArrayItem` (`PrimitiveComponent.GetOverlappingActors` (`self.Checker`) "Tile02_C")) "/Script/Engine.StaticMeshComponent" "Tile"))) "Static")
            ;[1 1 1] X UP 300
            (`SceneComponent.K2_SetWorldLocation` (`self.Checker`) (`KismetMathLibrary.MakeVector` (+ (.x (`SceneComponent.K2_GetComponentLocation` (`self.Checker`))) 300.0) (.y (`SceneComponent.K2_GetComponentLocation` (`self.Checker`))) (.z (`SceneComponent.K2_GetComponentLocation` (`self.Checker`)))) false false)
            ;[1 1 1] TILE????
            (if (`KismetStringLibrary.Contains` (`KismetSystemLibrary.GetDisplayName` (`|GetArrayItem` (`self.GetComponentsByTag` (`|GetArrayItem` (`PrimitiveComponent.GetOverlappingActors` (`self.Checker`) "Tile02_C")) "/Script/Engine.StaticMeshComponent" "Tile"))) "Static")
              ;[1 1 1] X UP 600
              (`SceneComponent.K2_SetWorldLocation` (`self.Checker`) (`KismetMathLibrary.MakeVector` (+ (.x (`SceneComponent.K2_GetComponentLocation` (`self.Checker`))) 300.0) (.y (`SceneComponent.K2_GetComponentLocation` (`self.Checker`))) (.z (`SceneComponent.K2_GetComponentLocation` (`self.Checker`)))) false false)
              (bind (_outactors_2 _returnvalue_2) (`KismetSystemLibrary.ComponentOverlapActors` _checker_4 (`SceneComponent.K2_GetComponentToWorld` _checker_4) (`self.TypeSelected`) "/Game/PuzzleBP/Blueprints/PC_BP.PC_BP_C"))
              ;[1 1 1] PLAYER???
              (if _returnvalue_2
                (set `self.Clickable` true)
                ;[1 1 1] SET MAT T/F
                (`PrimitiveComponent.SetMaterial` (`self.StaticMesh`) 0 "/Game/Puzzle/Meshes/BlueMaterial.BlueMaterial")
                (else
                  (`PrimitiveComponent.SetMaterial` (`self.StaticMesh`) 0 "/Game/Materials/M_Main_I_Tan.M_Main_I_Tan")
                  (`KismetSystemLibrary.PrintString` "" :!label _label_4)
                  ;[1 1 1] Y LEFT 300
                  (`SceneComponent.K2_SetWorldLocation` (`self.Checker`) (`KismetMathLibrary.MakeVector` (.x (`SceneComponent.K2_GetComponentLocation` (`self.DefaultSceneRoot`))) (+ (.y (`SceneComponent.K2_GetComponentLocation` (`self.DefaultSceneRoot`))) -300.0) (.z (`SceneComponent.K2_GetComponentLocation` (`self.DefaultSceneRoot`)))) false false)
                  (`KismetSystemLibrary.Delay` (`self.Delay`))
                  ;[1 1 1] TILE????
                  (if (`KismetStringLibrary.Contains` (`KismetSystemLibrary.GetDisplayName` (`|GetArrayItem` (`self.GetComponentsByTag` (`|GetArrayItem` (`PrimitiveComponent.GetOverlappingActors` (`self.Checker`) "Tile02_C")) "/Script/Engine.StaticMeshComponent" "Tile"))) "Static")
                    ;[1 1 1] X DOWN 300
                    (`SceneComponent.K2_SetWorldLocation` (`self.Checker`) (`KismetMathLibrary.MakeVector` (+ (.x (`SceneComponent.K2_GetComponentLocation` (`self.Checker`))) -300.0) (.y (`SceneComponent.K2_GetComponentLocation` (`self.Checker`))) (.z (`SceneComponent.K2_GetComponentLocation` (`self.Checker`)))) false false)
                    ;[1 1 1] TILE????
                    (if (`KismetStringLibrary.Contains` (`KismetSystemLibrary.GetDisplayName` (`|GetArrayItem` (`self.GetComponentsByTag` (`|GetArrayItem` (`PrimitiveComponent.GetOverlappingActors` (`self.Checker`) "Tile02_C")) "/Script/Engine.StaticMeshComponent" "Tile"))) "Static")
                      ;[1 1 1] X DOWN 600
                      (`SceneComponent.K2_SetWorldLocation` (`self.Checker`) (`KismetMathLibrary.MakeVector` (+ (.x (`SceneComponent.K2_GetComponentLocation` (`self.Checker`))) -300.0) (.y (`SceneComponent.K2_GetComponentLocation` (`self.Checker`))) (.z (`SceneComponent.K2_GetComponentLocation` (`self.Checker`)))) false false)
                      (bind (_outactors_3 _returnvalue_3) (`KismetSystemLibrary.ComponentOverlapActors` _checker_2 (`SceneComponent.K2_GetComponentToWorld` _checker_2) (`self.TypeSelected`) "/Game/PuzzleBP/Blueprints/PC_BP.PC_BP_C"))
                      ;[1 1 1] PLAYER???
                      (if _returnvalue_3
                        (set `self.Clickable` true)
                        ;[1 1 1] SET MAT T/F
                        (`PrimitiveComponent.SetMaterial` (`self.StaticMesh`) 0 "/Game/Puzzle/Meshes/BlueMaterial.BlueMaterial")
                        (else
                          (`PrimitiveComponent.SetMaterial` (`self.StaticMesh`) 0 "/Game/Materials/M_Main_I_Tan.M_Main_I_Tan")
                          (`KismetSystemLibrary.PrintString` "" :!label _label_5)
                          ;[1 1 1] Y LEFT 300
                          (`SceneComponent.K2_SetWorldLocation` (`self.Checker`) (`KismetMathLibrary.MakeVector` (.x (`SceneComponent.K2_GetComponentLocation` (`self.DefaultSceneRoot`))) (+ (.y (`SceneComponent.K2_GetComponentLocation` (`self.DefaultSceneRoot`))) -300.0) (.z (`SceneComponent.K2_GetComponentLocation` (`self.DefaultSceneRoot`)))) false false)
                          (`KismetSystemLibrary.Delay` (`self.Delay`))
                          ;[1 1 1] TILE????
                          (if (`KismetStringLibrary.Contains` (`KismetSystemLibrary.GetDisplayName` (`|GetArrayItem` (`self.GetComponentsByTag` (`|GetArrayItem` (`PrimitiveComponent.GetOverlappingActors` (`self.Checker`) "Tile02_C")) "/Script/Engine.StaticMeshComponent" "Tile"))) "Static")
                            ;[1 1 1] X UP 300
                            (`SceneComponent.K2_SetWorldLocation` (`self.Checker`) (`KismetMathLibrary.MakeVector` (+ (.x (`SceneComponent.K2_GetComponentLocation` (`self.Checker`))) 300.0) (.y (`SceneComponent.K2_GetComponentLocation` (`self.Checker`))) (.z (`SceneComponent.K2_GetComponentLocation` (`self.Checker`)))) false false)
                            ;[1 1 1] TILE????
                            (if (`KismetStringLibrary.Contains` (`KismetSystemLibrary.GetDisplayName` (`|GetArrayItem` (`self.GetComponentsByTag` (`|GetArrayItem` (`PrimitiveComponent.GetOverlappingActors` (`self.Checker`) "Tile02_C")) "/Script/Engine.StaticMeshComponent" "Tile"))) "Static")
                              ;[1 1 1] X UP 600
                              (`SceneComponent.K2_SetWorldLocation` (`self.Checker`) (`KismetMathLibrary.MakeVector` (+ (.x (`SceneComponent.K2_GetComponentLocation` (`self.Checker`))) 300.0) (.y (`SceneComponent.K2_GetComponentLocation` (`self.Checker`))) (.z (`SceneComponent.K2_GetComponentLocation` (`self.Checker`)))) false false)
                              (bind (_outactors_4 _returnvalue_4) (`KismetSystemLibrary.ComponentOverlapActors` _checker_3 (`SceneComponent.K2_GetComponentToWorld` _checker_3) (`self.TypeSelected`) "/Game/PuzzleBP/Blueprints/PC_BP.PC_BP_C"))
                              ;[1 1 1] PLAYER???
                              (if _returnvalue_4
                                (set `self.Clickable` true)
                                ;[1 1 1] SET MAT T/F
                                (`PrimitiveComponent.SetMaterial` (`self.StaticMesh`) 0 "/Game/Puzzle/Meshes/BlueMaterial.BlueMaterial")
                                (else
                                  (`PrimitiveComponent.SetMaterial` (`self.StaticMesh`) 0 "/Game/Materials/M_Main_I_Tan.M_Main_I_Tan")
                                  (`KismetSystemLibrary.PrintString` "" :!label _label_6)
                                  (`SceneComponent.K2_SetRelativeLocation` (`self.Checker`) (0.0 0.0 0.0) false false)))
                              (else
                                (`SceneComponent.K2_SetWorldLocation` (`self.Checker`) (`SceneComponent.K2_GetComponentLocation` (`self.DefaultSceneRoot`)) false false)
                                (goto _label_6)))
                            (else
                              (`SceneComponent.K2_SetWorldLocation` (`self.Checker`) (`SceneComponent.K2_GetComponentLocation` (`self.DefaultSceneRoot`)) false false)
                              (goto _label_6)))))
                      (else
                        (`SceneComponent.K2_SetWorldLocation` (`self.Checker`) (`SceneComponent.K2_GetComponentLocation` (`self.DefaultSceneRoot`)) false false)
                        (goto _label_5)))
                    (else
                      (`SceneComponent.K2_SetWorldLocation` (`self.Checker`) (`SceneComponent.K2_GetComponentLocation` (`self.DefaultSceneRoot`)) false false)
                      (goto _label_5)))))
              (else
                (`SceneComponent.K2_SetWorldLocation` (`self.Checker`) (`SceneComponent.K2_GetComponentLocation` (`self.DefaultSceneRoot`)) false false)
                (goto _label_4)))
            (else
              (`SceneComponent.K2_SetWorldLocation` (`self.Checker`) (`SceneComponent.K2_GetComponentLocation` (`self.DefaultSceneRoot`)) false false)
              (goto _label_4)))))
      (else
        (`SceneComponent.K2_SetWorldLocation` (`self.Checker`) (`SceneComponent.K2_GetComponentLocation` (`self.DefaultSceneRoot`)) false false)
        (goto _label_3)))
    (else
      (`SceneComponent.K2_SetWorldLocation` (`self.Checker`) (`SceneComponent.K2_GetComponentLocation` (`self.DefaultSceneRoot`)) false false)
      (goto _label_3))))

(event `self.ReceiveBeginPlay`
  (bind _aspuzzle_player_character (cast `/Game/PuzzleBP/Blueprints/PuzzlePlayerCharacter` (`GameplayStatics.GetPlayerPawn` 0)))
  ;[1 1 1] Y RIGHT 300
  (set `self.MuhCharacdor` _aspuzzle_player_character)
  (goto _label_2))

(event `self.Box.OnComponentBeginOverlap`
  (params (OverlappedComponent :type "PrimitiveComponent Object Reference") (OtherActor :type "Actor Object Reference") (OtherComp :type "PrimitiveComponent Object Reference") (OtherBodyIndex :type Integer) (bFromSweep :type Boolean) (SweepResult :type "HitResult Structure (by ref)")))

(fn `UserConstructionScript`)